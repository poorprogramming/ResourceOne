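; Celestial body actor for Mundus that spins around its vertical axis and feeds sun direction to materials.
; Tick advances the yaw through a delta-time math expression, applies it as the absolute rotation with zero pitch and roll, and stores the result.
; The construction script writes the sun actor's forward vector to a Material Parameter Collection, with a self-resetting RefreshSun toggle.
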(event EventBeginPlay)

(event Collision|EventActorBeginOverlap
  (params (OtherActor :type Actor%20Object%20Reference)))

(event EventTick
  (params (DeltaSeconds :type Float%20%28single-precision%29))
  (bind _output_get (Variables|Default|SetRot-Mundus (|((deltaseconds*{E167FCF7-40BA-94F3-9B5B-7788FD8D1122})+{095598FF-451C-7F59-B632-59B43C7790C8}) DeltaSeconds)))
  (Transformation|SetActorRotation (Math|Rotator|MakeRotator 0.0 0.0 _output_get))
  (Variables|Default|SetMundusRot (Transformation|GetActorRotation)))

(fn ConstructionScript
  (if (Variables|Default|GetRefreshSun)
    (Variables|Default|SetRefreshSun false))
  (Rendering|Material|SetVectorParameterValue "/Game/Blueprints/CelestialBodies/SunDirection.SunDirection" "LightDirection" (Math|Conversions|ToLinearColor(Vector) (Math|Rotator|GetRotationXVector (Transformation|GetActorRotation (Variables|Default|GetSunDirection)))) :!class /Script/Engine.KismetMaterialLibrary))