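; Solar system actor that animates the orbit and spin of Mundus, Bellum and their moons.
; Tick advances per-body angles at DevTime-scaled rates, rotating pivot components for orbits; moon pivots follow Mundus (Satalite) or Bellum (Gladio, Armis, Credo).
; Overlapping Mundus slows the HomoCommander camera, reached through the game instance, until exit.
; The construction script writes SolarDirection's forward vector to a material parameter collection as light direction and disables StarSphere shadows.
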(event OnComponentBeginOverlap(Mundus)
  (params (OverlappedComponent :type Primitive%20Component%20Object%20Reference) (OtherActor :type Actor%20Object%20Reference) (OtherComp :type Primitive%20Component%20Object%20Reference) (OtherBodyIndex :type Integer) (bFromSweep :type Boolean) (SweepResult :type Hit%20Result%20Structure%20%28by%20ref%29))
  (bind _ashomo_commander (Utilities|Casting|CastToHomoCommander (Variables|/Game/Blueprints/Logic/ResourceGameInstance.ResourceGameInstance_C|GetHomoCommander (Variables|Game|GetGI_Resource))))
  (Variables|/Game/Blueprints/A_Units/HomoCommander.HomoCommander_C|SetCamera_MoveSpeed _ashomo_commander 1e+01)
  (Development|PrintString "ENTERRRRRRRRRR"))

(event OnComponentEndOverlap(Mundus)
  (params (OverlappedComponent :type Primitive%20Component%20Object%20Reference) (OtherActor :type Actor%20Object%20Reference) (OtherComp :type Primitive%20Component%20Object%20Reference) (OtherBodyIndex :type Integer))
  (bind _ashomo_commander (Utilities|Casting|CastToHomoCommander (Variables|/Game/Blueprints/Logic/ResourceGameInstance.ResourceGameInstance_C|GetHomoCommander (Variables|Game|GetGI_Resource))))
  (Variables|/Game/Blueprints/A_Units/HomoCommander.HomoCommander_C|SetCamera_MoveSpeed _ashomo_commander 1e+02)
  (Development|PrintString "TREXITMMM MY EXIT"))

(event EventBeginPlay
  (bind _dev_time (Variables|Default|GetDev_Time))
  (bind _asresource_game_instance (Utilities|Casting|CastToResourceGameInstance (Game|GetGameInstance)))
  (Variables|Game|SetGI_Resource _asresource_game_instance)
  (Utilities|FlowControl|Sequence
    (:then_0
      ;[1 1 1] Dev_Setting - Time
      (Variables|Default|SetOrbit_MultiMundus (* _dev_time (Variables|Default|GetOrbit_MultiMundus)))
      (Variables|Default|SetOrbit_MultiSatalite (* _dev_time (Variables|Default|GetOrbit_MultiSatalite)))
      (Variables|Default|SetOrbit_MultiBellum (* _dev_time (Variables|Default|GetOrbit_MultiBellum)))
      (Variables|Default|SetOrbit_MultiGladio (* _dev_time (Variables|Default|GetOrbit_MultiGladio)))
      (Variables|Default|SetOrbit_MultiArmis (* _dev_time (Variables|Default|GetOrbit_MultiArmis)))
      (Variables|Default|SetOrbit_MultiCredo (* _dev_time (Variables|Default|GetOrbit_MultiCredo)))
      (Variables|Default|SetRot_MultiMundus (* _dev_time (Variables|Default|GetRot_MultiMundus)))
      (Variables|Default|SetRot_MultiBellum (* _dev_time (Variables|Default|GetRot_MultiBellum)))
      (Variables|Default|SetRot_MultiSatalite (* _dev_time (Variables|Default|GetRot_MultiSatalite)))
      (Variables|Default|SetRot_MultiGladio (* _dev_time (Variables|Default|GetRot_MultiGladio)))
      (Variables|Default|SetRot_MultiArmis (* _dev_time (Variables|Default|GetRot_MultiArmis)))
      (Variables|Default|SetRot_MultiCredo (* _dev_time (Variables|Default|GetRot_MultiCredo))))))

(event EventTick
  (params (DeltaSeconds :type Float%20%28single-precision%29))
  ;[1 1 1] Orbit And Rotation
  ;;[1 1 1] Orbit
  ;;;[1 1 1] Mundus
  (bind _output_get (Variables|Default|SetRot_OrbitMundus (|((deltaseconds*{A83DA565-473C-5DEC-0595-8EB1F3AFF640})+{0FFD4950-46DD-ECD9-CC54-A1978929ACEB}) DeltaSeconds)))
  (Transformation|SetWorldRotation (Variables|Default|GetRot_Mundus) (Math|Rotator|MakeRotator 0.0 0.0 _output_get) false false)
  ;;;[1 1 1] Bellum
  (bind _output_get_2 (Variables|Default|SetRot_OrbitBellum (|((deltaseconds*{63903912-48C3-CB4B-B2D4-70B94ECA0078})+{8F711784-4DAA-CBF8-215C-3FB0D854F05C}) DeltaSeconds)))
  (Transformation|SetWorldRotation (Variables|Default|GetRot_Bellum) (Math|Rotator|MakeRotator 0.0 _output_get_2 0.0) false false)
  ;;;[1 1 1] Satalite
  (bind _output_get_3 (Variables|Default|SetRot_OrbitSatalite (|((deltaseconds*{0B5AFFF3-44C7-081F-BCB9-36B2B18F8552})+{4307842E-4BF2-D132-6CF5-B99AA8A86B98}) DeltaSeconds)))
  (Transformation|SetWorldRotation (Variables|Default|GetRot_Satalite) (Math|Rotator|MakeRotator 0.0 0.0 _output_get_3) false false)
  (Transformation|SetWorldLocation (Variables|Default|GetRot_Satalite) (Transformation|GetWorldLocation (Variables|Default|GetMundus)) false false)
  ;;;[1 1 1] Gladio
  (bind _output_get_4 (Variables|Default|SetRot_OrbitGladio (|((deltaseconds*{C3E43C4F-4A16-566E-5F88-46990DC978FD})+{20266209-4501-C5E1-A6C3-7D89F6FEA522}) DeltaSeconds)))
  (Transformation|SetWorldRotation (Variables|Default|GetRot_Gladio) (Math|Rotator|MakeRotator 0.0 0.0 _output_get_4) false false)
  (Transformation|SetWorldLocation (Variables|Default|GetRot_Gladio) (Transformation|GetWorldLocation (Variables|Default|GetBellum)) false false)
  ;;;[1 1 1] Armis
  (bind _output_get_5 (Variables|Default|SetRot_OrbitArmis (|((deltaseconds*{2EEDC6FD-428E-53B6-C2F0-0EAD796DB1B2})+{0FB42DA6-40EF-E7C7-F91E-55BAB74204C0}) DeltaSeconds)))
  (Transformation|SetWorldRotation (Variables|Default|GetRot_Armis) (Math|Rotator|MakeRotator 0.0 _output_get_5 0.0) false false)
  (Transformation|SetWorldLocation (Variables|Default|GetRot_Armis) (Transformation|GetWorldLocation (Variables|Default|GetBellum)) false false)
  ;;;[1 1 1] Credo
  (bind _output_get_6 (Variables|Default|SetRot_OrbitCredo (|((deltaseconds*{A3E0F749-4D56-6DAF-7F58-48A9130DE3FD})+{A8513CAE-4AC8-0DBF-84CD-3EB161B180DA}) DeltaSeconds)))
  (Transformation|SetWorldRotation (Variables|Default|GetRot_Credo) (Math|Rotator|MakeRotator 0.0 _output_get_6 _output_get_6) false false)
  (Transformation|SetWorldLocation (Variables|Default|GetRot_Credo) (Transformation|GetWorldLocation (Variables|Default|GetBellum)) false false)
  ;;[1 1 1] Rotate
  ;;;[1 1 1] Mundus
  (bind _output_get_7 (Variables|Default|SetRot_OrbitMundus_0 (|((deltaseconds*{0C9A0D4B-4E15-9DB2-4111-81A42FA47FB7})+{A88FEA63-4B4A-B211-6448-23968516858C}) DeltaSeconds)))
  (Transformation|SetWorldRotation (Variables|Default|GetMundus) (Math|Rotator|MakeRotator 0.0 0.0 _output_get_7) false false)
  ;;;[1 1 1] Bellum
  (bind _output_get_8 (Variables|Default|SetRot_OrbitBellum_0 (|((deltaseconds*{0DBB855F-4157-D27D-620B-AFBC67889D5B})+{1D5B0FE9-49CC-1602-099F-BE937E2512E1}) DeltaSeconds)))
  (Transformation|SetWorldRotation (Variables|Default|GetBellum) (Math|Rotator|MakeRotator 0.0 _output_get_8 0.0) false false)
  ;;;[1 1 1] Satalite
  (bind _output_get_9 (Variables|Default|SetRot_OrbitSatalite_0 (|((deltaseconds*{EEDF8424-4951-C745-3975-56A218D96DAA})+{FC489B37-4C1F-16C7-BD8C-919FF28F3E0C}) DeltaSeconds)))
  (Transformation|SetWorldRotation (Variables|Default|GetSatalite) (Math|Rotator|MakeRotator 0.0 0.0 _output_get_9) false false)
  ;;;[1 1 1] Gladio
  (bind _output_get_10 (Variables|Default|SetRot_OrbitGladio_0 (|((deltaseconds*{C03AF68F-4EBC-5528-5187-44BA8598B363})+{2EB0DD0D-4FE9-E3FD-DD6E-FE9AC5A07740}) DeltaSeconds)))
  (Transformation|SetWorldRotation (Variables|Default|GetGladio) (Math|Rotator|MakeRotator 0.0 0.0 _output_get_10) false false)
  ;;;[1 1 1] Armis
  (bind _output_get_11 (Variables|Default|SetRot_OrbitArmis_0 (|((deltaseconds*{617B0EA7-4DA8-5DAB-2B17-389AF276B6B1})+{DE40E27B-4F7D-BF50-0817-3B95AE834B01}) DeltaSeconds)))
  (Transformation|SetWorldRotation (Variables|Default|GetArmis) (Math|Rotator|MakeRotator 0.0 _output_get_11 0.0) false false)
  ;;;[1 1 1] Credo
  (bind _output_get_12 (Variables|Default|SetRot_OrbitCredo_0 (|((deltaseconds*{91D09AA6-4685-51F0-DC4B-5196C46856AB})+{EA711C04-43B9-173B-D5FF-68A77E99AF24}) DeltaSeconds)))
  (Transformation|SetWorldRotation (Variables|Default|GetCredo) (Math|Rotator|MakeRotator 0.0 _output_get_12 _output_get_12) false false))

(fn ConstructionScript
  (if (Variables|Default|GetRefresh_Solar)
    (Variables|Default|SetRefresh_Solar false))
  (Rendering|Material|SetVectorParameterValue "/Game/Materials/CelestialBodies/MPC_SolarOneDirection.MPC_SolarOneDirection" "LightDirection" (Math|Conversions|ToLinearColor(Vector) (Math|Rotator|GetRotationXVector (Transformation|GetActorRotation (Variables|Default|GetSolar%20Direction)))) :!class /Script/Engine.KismetMaterialLibrary)
  (Rendering|SetCastShadow (Variables|Default|GetStarSphere) false))