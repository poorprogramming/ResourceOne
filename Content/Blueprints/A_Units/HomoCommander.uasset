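; Player commander pawn that flies a build camera, creates the in-game HUD and registers both with ResourceGameInstance.
; Axis inputs move it, keys and wheel shift height, and right-mouse drag pans or rotates depending on CameraTPanFRotate.
; A ghost building follows the cursor trace on a 0.01-second Delay loop; a valid left click asks it to spawn the real building.
; ROS_SpawnActualBuilding spawns that building with its commander reference.
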(event `self.ReceiveBeginPlay`
  (`self.StartUp`))

(event `self.ReceiveTick`
  (params (DeltaSeconds :type "Float (single-precision)"))
  (if (`self.InStrongOrbit`)
    _))

(event `InputAxis|MoveForward`
  (params (AxisValue :type "Float (single-precision)"))
  ;[1 1 1] Camera Directional Movement
  (`self.Camera_MoveDirections` AxisValue (stale `InputAxis|MoveRight` AxisValue) (stale `InputAxis|MoveUp` AxisValue) :!label _label))

(event `BuildGhostBuilding`
  (params (InBuildButton :type "UserWidget Object Reference") (InBuilding :type "/Game/Blueprints/A_Units/M_GhostBuilding Class Reference"))
  ;[1 1 1] Building Placement
  (`self.SpawnGhostBuilding` InBuildButton InBuilding)
  (`self.GhostBuildingFollowMouse` :!label _label_2))

(event `Key|LeftMouseButton`
  (params (Key :type "Key Structure" :default "AnyKey"))
  (:`Pressed`
    (if (`self.PlacingBuilding`)
      (`self.BuildingPlaced`))))

(event `InputAxis|MoveRight`
  (params (AxisValue :type "Float (single-precision)"))
  ;[1 1 1] Camera Directional Movement
  (goto _label :!via `LeftAndRight`))

(event `BuildingPlaced`
  ;[1 1 1] Building Placement
  (goto _label_2 :!via `BuildingPlaced`))

(event `Key|RightMouseButton`
  (params (Key :type "Key Structure" :default "AnyKey"))
  (:`Pressed`
    (if (`self.PlacingBuilding`)
      (`self.K2_DestroyActor` (`self.GhostBuilding`)))))

(event `InputAxis|MoveUp`
  (params (AxisValue :type "Float (single-precision)"))
  ;[1 1 1] Camera Directional Movement
  (goto _label :!via `UpAndDown`))

(event `DestroyGhost`
  ;[1 1 1] Building Placement
  (goto _label_2 :!via `DestroyGhost`))

(event `ROS_SpawnActualBuilding`
  (params (InBuilding :type "/Game/Blueprints/A_Units/M_Building Class Reference") (InTransform :type "Transform Structure") (InCommander :type "Pawn Object Reference"))
  ;[1 1 1] Building Placement
  (`self.SpawnActualBuilding` InBuilding InTransform InCommander))

(event `Key|SpaceBar`
  (params (Key :type "Key Structure" :default "AnyKey"))
  ;[1 1 1] Camera Zoom
  (:`Pressed`
    (`self.Camera_Zoom` :!label _label_3)))

(event `Key|MouseScrollUp`
  (params (Key :type "Key Structure" :default "AnyKey"))
  ;[1 1 1] Camera Zoom
  (:`Pressed`
    (goto _label_3)))

(event `Key|LeftControl`
  (params (Key :type "Key Structure" :default "AnyKey"))
  ;[1 1 1] Camera Zoom
  (:`Pressed`
    (goto _label_3 :!via `MoveDown`)))

(event `Key|MouseScrollDown`
  (params (Key :type "Key Structure" :default "AnyKey"))
  ;[1 1 1] Camera Zoom
  (:`Pressed`
    (goto _label_3 :!via `MoveDown`)))

(event `InputAxisKey|MouseX`
  (params (AxisValue :type "Float (single-precision)"))
  ;[1 1 1] Camera Pan/Rotate
  (`/Engine/EditorBlueprintResources/StandardMacros.Gate` true :!label _label_4
    (:`Exit`
      (if (`self.Camera_TPanFRotate`)
        (`self.Camera_Pan` AxisValue (stale `InputAxisKey|MouseY` AxisValue) :!label _label_5)
        (else
          (`self.Camera_Rotate` AxisValue (stale `InputAxisKey|MouseY` AxisValue) :!label _label_6))))))

(event `Key|RightMouseButton`
  (params (Key :type "Key Structure" :default "AnyKey"))
  ;[1 1 1] Camera Pan/Rotate
  (:`Pressed`
    (`|ExecutionSequence`
      (:`then_0`
        (goto _label_4 :!via `Open`))
      (:`then_1`
        (goto _label_7 :!via `Open`))))
  (:`Released`
    (`|ExecutionSequence`
      (:`then_0`
        (goto _label_4 :!via `Close`))
      (:`then_1`
        (goto _label_7 :!via `Close`)))))

(event `InputAxisKey|MouseY`
  (params (AxisValue :type "Float (single-precision)"))
  ;[1 1 1] Camera Pan/Rotate
  (`/Engine/EditorBlueprintResources/StandardMacros.Gate` true :!label _label_7
    (:`Exit`
      (if (`self.Camera_TPanFRotate`)
        (goto _label_5 :!via `MouseY`)
        (else
          (goto _label_6 :!via `MouseY`))))))

(fn `CreateWidgets`
  (bind _returnvalue (`|CreateWidget` "/Game/Blueprints/UI/UI_InGame.UI_InGame_C" null self))
  (bind _output_get (set `self.CommanderHUD` _returnvalue))
  (bind _asresource_game_instance (cast `/Game/Blueprints/Logic/ResourceGameInstance` (`GameplayStatics.GetGameInstance`)))
  (bind _output_get_2 (set `/Game/Blueprints/Logic/ResourceGameInstance.CommanderHUD` _output_get _asresource_game_instance))
  (`UserWidget.AddToViewport` _output_get_2 0))

(fn `SetGameInstanceVariable`
  (bind _asresource_game_instance (cast `/Game/Blueprints/Logic/ResourceGameInstance` (`GameplayStatics.GetGameInstance`)))
  (set `/Game/Blueprints/Logic/ResourceGameInstance.Commander` self _asresource_game_instance)
  (set `/Game/Blueprints/Logic/ResourceGameInstance.CommanderHUD` (`self.CommanderHUD`) _asresource_game_instance))

(fn `SpawnActualBuilding`
  (params (InBuilding :type "/Game/Blueprints/A_Units/M_Building Class Reference") (InTransform :type "Transform Structure") (InCommander :type "Pawn Object Reference"))
  (`|SpawnActorFromClass` InBuilding InTransform "Undefined" "OverrideRootScale" null InCommander))

(fn `SpawnGhostBuilding`
  (params (InBuildingButton :type "UserWidget Object Reference") (InBuilding :type "/Game/Blueprints/A_Units/M_GhostBuilding Class Reference"))
  (set `self.PlacingBuilding` true)
  (set `self.BuildButton` InBuildingButton)
  (bind _returnvalue (`|SpawnActorFromClass` InBuilding (`KismetMathLibrary.Conv_VectorToTransform` (`.Location` (`GameplayStatics.BreakHitResult` (`PlayerController.GetHitResultUnderCursorByChannel` (`GameplayStatics.GetPlayerController` 0) "TraceTypeQuery1" true)))) "Undefined" "OverrideRootScale" null self))
  (set `self.GhostBuilding` _returnvalue))

(fn `StartUp`
  (set `PlayerController.bShowMouseCursor` true (`GameplayStatics.GetPlayerController` 0))
  (`self.CreateWidgets`)
  (`self.SetGameInstanceVariable`))

(fn `UserConstructionScript`)